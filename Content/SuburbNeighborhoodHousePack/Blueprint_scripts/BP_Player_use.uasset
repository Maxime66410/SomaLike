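; BP_Player_use is a helper Blueprint that lets the player open and close doors with the E key.
; On BeginPlay it enables input from the first player controller and prints an on-screen key hint.
; Pressing E traces a short line forward from the player character's camera on the Camera channel, ignoring the character.
; If the hit actor is a main or garage door, it calls that door's OpenClose.
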(event EventBeginPlay
  (Input|EnableInput (Game|GetPlayerController 0))
  (Development|PrintString "Press E to open/close doors with 1st or 3rd person controller" true true "(R=0.000000,G=0.660000,B=1.000000,A=1.000000)" 5.0))

(event Input|KeyboardEvents|E
  (params (Key :type Key%20Structure :default "None"))
  (bind _returnvalue (Game|GetPlayerCharacter 0))
  (bind _returnvalue_2 (Actor|GetComponentbyClass _returnvalue "/Script/Engine.CameraComponent"))
  (bind _returnvalue_3 (Transformation|GetWorldLocation _returnvalue_2))
  (:Pressed
    (if (Utilities|IsValid _returnvalue)
      (bind _outhit (Collision|LineTraceByChannel _returnvalue_3 (+ _returnvalue_3 (* (Math|Vector|GetForwardVector _returnvalue_2) 5e+02)) "TraceTypeQuery2" false (Utilities|Array|MakeArray _returnvalue) "None"))
      (Utilities|FlowControl|Sequence
        (:then_0
          (bind _asbp_door_main (Utilities|Casting|CastToBP_Door_main (.HitActor (Collision|BreakHitResult _outhit))))
          (Default|OpenClose _asbp_door_main))
        (:then_1
          (bind _asbp_door_garage (Utilities|Casting|CastToBP_Door_garage (.HitActor (Collision|BreakHitResult _outhit))))
          (Default|OpenClose _asbp_door_garage))))))

(fn ConstructionScript)