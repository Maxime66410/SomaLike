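; BP_Floors is a modular house-building actor that places a selectable floor piece with an optional matching ceiling.
; The construction script picks both meshes from arrays using the Floors selection, raises the ceiling by 300 units, and destroys whichever component is toggled off.
; A RevertDefaultMaterials flag acts as a one-shot editor button that restores each mesh's default materials, then clears itself.
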(event EventBeginPlay)

(event Collision|EventActorBeginOverlap
  (params (OtherActor :type Actor%20Object%20Reference)))

(event EventTick
  (params (DeltaSeconds :type Float%20%28single-precision%29)))

(fn ConstructionScript
  (bind _floor_meshes (Variables|Mesh|GetFloor%20Meshes))
  (bind _ceiling_mesh (Variables|Default|GetCeiling_mesh))
  (bind _floor_mesh (Variables|Default|GetFloor_mesh))
  (bind _floors (Variables|Mesh|GetFloors))
  (bind _returnvalue (Math|Conversions|ToInteger(Byte) _floors))
  (bind _output (Utilities|Array|Get(acopy) _floor_meshes _returnvalue))
  (if (Variables|Mesh|GetAdd%20Floor)
    _
    (else
      (Components|DestroyComponent (Variables|Default|GetFloor_mesh))))
  (Components|StaticMesh|SetStaticMesh (Variables|Default|GetFloor_mesh) _output)
  (LocalVariables|SetNew_mesh _output)
  (if (Variables|Mesh|GetAdd%20Ceiling)
    (Components|StaticMesh|SetStaticMesh (Variables|Default|GetCeiling_mesh) (Utilities|Array|Get(acopy) (Variables|Mesh|GetCeiling%20Meshes) _returnvalue))
    (Transformation|AddLocalOffset (Variables|Default|GetCeiling_mesh) "0, 0,300.000000" false false)
    (else
      (Components|DestroyComponent (Variables|Default|GetCeiling_mesh))))
  (if (Variables|Mesh|GetRevert%20Default%20Materials)
    (Utilities|FlowControl|Sequence
      (:then_0
        (bind _output_get (LocalVariables|SetNumber%20Of%20Materials (Rendering|Material|GetNumMaterials _ceiling_mesh)))
        (for _index (range 0 _output_get)
          (Rendering|Material|SetMaterial _ceiling_mesh _index (Rendering|Material|GetMaterial (Variables|/Script/Engine.StaticMeshComponent|GetStaticMesh _ceiling_mesh) _index)))
        (Variables|Mesh|SetRevert%20Default%20Materials false))
      (:then_1
        (bind _output_get_2 (LocalVariables|SetNumber%20Of%20Materials (Rendering|Material|GetNumMaterials _floor_mesh)))
        (for _index_2 (range 0 _output_get_2)
          (Rendering|Material|SetMaterial _floor_mesh _index_2 (Rendering|Material|GetMaterial (LocalVariables|GetNew_mesh) _index_2)))
        (Variables|Mesh|SetRevert%20Default%20Materials false)))))