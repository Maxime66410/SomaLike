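; Modular first-floor wall piece for suburban houses, assembled entirely in the construction script from the Walls1stFloor enum.
; The enum picks the wall mesh, matching window glass and optional window blocker with its offset, destroying components a variant does not use.
; The openable-window variant adds a sash whose height follows the WindowOpenable value.
; RevertDefaultMaterials acts as an editor button, restoring the mesh's default materials and then resetting itself.
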(event EventBeginPlay)

(event Collision|EventActorBeginOverlap
  (params (OtherActor :type Actor%20Object%20Reference)))

(event EventTick
  (params (DeltaSeconds :type Float%20%28single-precision%29)))

(fn ConstructionScript
  (bind _window_blocker_mesh (Variables|Default|GetWindow_blocker_mesh))
  (bind _walls_1st_floor (Variables|Mesh|GetWalls_1st_floor))
  (bind _wall_mesh (Variables|Default|GetWall_mesh))
  (bind _walls_1st_floor_meshes (Variables|Mesh|GetWalls%201st%20Floor%20Meshes))
  (bind _windowglass (Variables|Default|GetWindowglass))
  (bind _returnvalue (Math|Conversions|ToInteger(Byte) _walls_1st_floor))
  (bind _output (Utilities|Array|Get(acopy) _walls_1st_floor_meshes _returnvalue))
  (Components|StaticMesh|SetStaticMesh (Variables|Default|GetWall_mesh) _output)
  (LocalVariables|SetNew_mesh _output)
  (Math|Integer|CompareInt _returnvalue 19
    (:>
      (Components|DestroyComponent (Variables|Default|GetWindow_openable) :!label _label))
    (:==
      (Components|StaticMesh|SetStaticMesh (Variables|Default|GetWindow_openable) "/Game/SuburbNeighborhoodHousePack/Meshes/Meshes_construction/SM_Window_openable.SM_Window_openable")
      (Class|KismetMathLibrary|VectorSet (Variables|Mesh|GetWindow%20open%20location) 0.0 1.5e+02 (Math|Float|MapRangeClamped (Variables|Mesh|GetWindow%20openable) 0.0 1.0 1.8e+02 2.4e+02))
      (Transformation|SetRelativeLocation (Variables|Default|GetWindow_openable) (Variables|Mesh|GetWindow%20open%20location) false false))
    (:<
      (goto _label)))
  (switch Utilities|FlowControl|Switch|SwitchonE_Walls_1st_floor (Variables|Mesh|GetWalls_1st_floor)
    (:NewEnumerator19
      (Components|DestroyComponent _windowglass :!label _label_2))
    (:NewEnumerator5
      (goto _label_2))
    (:NewEnumerator6
      (goto _label_2))
    (:NewEnumerator7
      (goto _label_2))
    (:NewEnumerator8
      (goto _label_2))
    (:NewEnumerator23
      (goto _label_2))
    (:NewEnumerator9
      (goto _label_2))
    (:NewEnumerator24
      (goto _label_2))
    (:NewEnumerator2
      (goto _label_2))
    (:NewEnumerator20
      (goto _label_2))
    (:NewEnumerator3
      (Components|StaticMesh|SetStaticMesh _windowglass "/Game/SuburbNeighborhoodHousePack/Meshes/Meshes_construction/SM_Wall_1st_3x_door_B_windowglass.SM_Wall_1st_3x_door_B_windowglass")
      (Transformation|SetRelativeLocation _windowglass "0, 0, 0" false false :!label _label_3))
    (:NewEnumerator4
      (Components|StaticMesh|SetStaticMesh _windowglass "/Game/SuburbNeighborhoodHousePack/Meshes/Meshes_construction/SM_Wall_1st_3x_door_C_windowglass.SM_Wall_1st_3x_door_C_windowglass")
      (goto _label_3))
    (:NewEnumerator10
      (Components|StaticMesh|SetStaticMesh _windowglass "/Game/SuburbNeighborhoodHousePack/Meshes/Meshes_construction/SM_Wall_1st_3x_window_double_A_windowglass.SM_Wall_1st_3x_window_double_A_windowglass")
      (goto _label_3))
    (:NewEnumerator11
      (Components|StaticMesh|SetStaticMesh _windowglass "/Game/SuburbNeighborhoodHousePack/Meshes/Meshes_construction/SM_Wall_1st_3x_window_double_B_windowglass.SM_Wall_1st_3x_window_double_B_windowglass")
      (goto _label_3))
    (:NewEnumerator12
      (Components|StaticMesh|SetStaticMesh _windowglass "/Game/SuburbNeighborhoodHousePack/Meshes/Meshes_construction/SM_Wall_1st_3x_window_double_C_windowglass.SM_Wall_1st_3x_window_double_C_windowglass")
      (goto _label_3))
    (:NewEnumerator14
      (Components|StaticMesh|SetStaticMesh _windowglass "/Game/SuburbNeighborhoodHousePack/Meshes/Meshes_construction/SM_Wall_1st_3x_window_single_A_windowglass.SM_Wall_1st_3x_window_single_A_windowglass")
      (goto _label_3))
    (:NewEnumerator15
      (Components|StaticMesh|SetStaticMesh _windowglass "/Game/SuburbNeighborhoodHousePack/Meshes/Meshes_construction/SM_Wall_1st_3x_window_single_B_windowglass.SM_Wall_1st_3x_window_single_B_windowglass")
      (goto _label_3))
    (:NewEnumerator16
      (Components|StaticMesh|SetStaticMesh _windowglass "/Game/SuburbNeighborhoodHousePack/Meshes/Meshes_construction/SM_Wall_1st_3x_window_single_C_windowglass.SM_Wall_1st_3x_window_single_C_windowglass")
      (goto _label_3))
    (:NewEnumerator22
      (Components|StaticMesh|SetStaticMesh _windowglass "/Game/SuburbNeighborhoodHousePack/Meshes/Meshes_construction/SM_Wall_1st_3x_window_single_D_windowglass.SM_Wall_1st_3x_window_single_D_windowglass")
      (goto _label_3))
    (:NewEnumerator13
      (Components|StaticMesh|SetStaticMesh _windowglass "/Game/SuburbNeighborhoodHousePack/Meshes/Meshes_construction/SM_Wall_1st_3x_window_openable_windowglass.SM_Wall_1st_3x_window_openable_windowglass")
      (goto _label_3))
    (:NewEnumerator17
      (Components|StaticMesh|SetStaticMesh _windowglass "/Game/SuburbNeighborhoodHousePack/Meshes/Meshes_construction/SM_Wall_1st_3x_window_bay_A_windowglass.SM_Wall_1st_3x_window_bay_A_windowglass")
      (goto _label_3))
    (:NewEnumerator18
      (Components|StaticMesh|SetStaticMesh _windowglass "/Game/SuburbNeighborhoodHousePack/Meshes/Meshes_construction/SM_Wall_1st_3x_window_bay_B_windowglass.SM_Wall_1st_3x_window_bay_B_windowglass")
      (goto _label_3))
    (:NewEnumerator21
      (Components|StaticMesh|SetStaticMesh _windowglass "/Game/SuburbNeighborhoodHousePack/Meshes/Meshes_construction/SM_Wall_1st_4x_window_double_windowglass.SM_Wall_1st_4x_window_double_windowglass")
      (goto _label_3))
    (:NewEnumerator0
      (goto _label_2))
    (:NewEnumerator1
      (goto _label_2)))
  (if (Variables|Mesh|GetWindow_blocker)
    (switch int _returnvalue
      (:Default
        (Components|DestroyComponent (Variables|Default|GetWindow_blocker_mesh) :!label _label_4))
      (:10
        (Components|StaticMesh|SetStaticMesh _window_blocker_mesh "/Game/SuburbNeighborhoodHousePack/Meshes/Meshes_construction/SM_Window_blocker_Wall_1st_3x_door_B.SM_Window_blocker_Wall_1st_3x_door_B")
        (Transformation|SetRelativeLocation _window_blocker_mesh "15.000000,150.000000,180.000000" false false))
      (:11
        (Components|StaticMesh|SetStaticMesh _window_blocker_mesh "/Game/SuburbNeighborhoodHousePack/Meshes/Meshes_construction/SM_Window_blocker_Wall_1st_3x_door_C.SM_Window_blocker_Wall_1st_3x_door_C")
        (Transformation|SetRelativeLocation _window_blocker_mesh "15.000000,150.000000,180.000000" false false))
      (:12
        (Components|StaticMesh|SetStaticMesh _window_blocker_mesh "/Game/SuburbNeighborhoodHousePack/Meshes/Meshes_construction/SM_Window_blocker_A.SM_Window_blocker_A" :!label _label_5)
        (Transformation|SetRelativeLocation _window_blocker_mesh "15.000000,150.000000,180.000000" false false))
      (:13
        (goto _label_5))
      (:14
        (goto _label_5))
      (:15
        (goto _label_5))
      (:16
        (goto _label_5))
      (:17
        (Components|StaticMesh|SetStaticMesh _window_blocker_mesh "/Game/SuburbNeighborhoodHousePack/Meshes/Meshes_construction/SM_Window_blocker_B.SM_Window_blocker_B" :!label _label_6)
        (Transformation|SetRelativeLocation _window_blocker_mesh "15.000000,150.000000,180.000000" false false))
      (:18
        (goto _label_6))
      (:19
        (goto _label_6))
      (:20
        (Components|StaticMesh|SetStaticMesh _window_blocker_mesh "/Game/SuburbNeighborhoodHousePack/Meshes/Meshes_construction/SM_Window_blocker_A.SM_Window_blocker_A")
        (Transformation|SetRelativeLocation _window_blocker_mesh "-35.000000,150.000000,180.000000" false false))
      (:21
        (Components|StaticMesh|SetStaticMesh _window_blocker_mesh "/Game/SuburbNeighborhoodHousePack/Meshes/Meshes_construction/SM_Window_blocker_Wall_1st_3x_window_bay_B.SM_Window_blocker_Wall_1st_3x_window_bay_B")
        (Transformation|SetRelativeLocation _window_blocker_mesh "15.000000,150.000000,180.000000" false false))
      (:22
        (Components|StaticMesh|SetStaticMesh _window_blocker_mesh "/Game/SuburbNeighborhoodHousePack/Meshes/Meshes_construction/SM_Window_blocker_A.SM_Window_blocker_A")
        (Transformation|SetRelativeLocation _window_blocker_mesh "15.000000,200.000000,180.000000" false false)))
    (else
      (goto _label_4)))
  (if (Variables|Mesh|GetRevert%20Default%20Materials)
    (bind _output_get (LocalVariables|SetNumber%20Of%20Materials (Rendering|Material|GetNumMaterials _wall_mesh)))
    (for _index (range 0 _output_get)
      (Rendering|Material|SetMaterial _wall_mesh _index (Rendering|Material|GetMaterial (LocalVariables|GetNew_mesh) _index)))
    (Variables|Mesh|SetRevert%20Default%20Materials false)))