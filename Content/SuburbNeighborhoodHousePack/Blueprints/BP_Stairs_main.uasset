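; Stairs actor for the suburban house pack, configured through its construction script with no active gameplay logic.
; The FloorsCeiling selection picks the floor/ceiling mesh from the FloorMeshes array.
; RevertDefaultMaterials works as a one-shot toggle that restores every material slot on the stairs and floor/ceiling meshes from their static mesh assets, then clears itself.
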(event EventBeginPlay)

(event Collision|EventActorBeginOverlap
  (params (OtherActor :type Actor%20Object%20Reference)))

(event EventTick
  (params (DeltaSeconds :type Float%20%28single-precision%29)))

(fn ConstructionScript
  (bind _floors_ceiling (Variables|Mesh|GetFloors_ceiling))
  (bind _stairs_main (Variables|Default|GetStairs_main))
  (bind _floor_meshes (Variables|Mesh|GetFloor%20Meshes))
  (bind _floorceiling_mesh (Variables|Default|GetFloorCeiling_mesh))
  (bind _returnvalue (Math|Conversions|ToInteger(Byte) _floors_ceiling))
  (bind _output (Utilities|Array|Get(acopy) _floor_meshes _returnvalue))
  (Components|StaticMesh|SetStaticMesh (Variables|Default|GetFloorCeiling_mesh) _output)
  (LocalVariables|SetNew_mesh _output)
  (if (Variables|Mesh|GetRevert%20Default%20Materials)
    (Utilities|FlowControl|Sequence
      (:then_0
        (bind _output_get (LocalVariables|SetNumber%20Of%20Materials (Rendering|Material|GetNumMaterials _stairs_main)))
        (for _index (range 0 _output_get)
          (Rendering|Material|SetMaterial _stairs_main _index (Rendering|Material|GetMaterial (Variables|/Script/Engine.StaticMeshComponent|GetStaticMesh _stairs_main) _index)))
        (Variables|Mesh|SetRevert%20Default%20Materials false))
      (:then_1
        (bind _output_get_2 (LocalVariables|SetNumber%20Of%20Materials (Rendering|Material|GetNumMaterials _floorceiling_mesh)))
        (for _index_2 (range 0 _output_get_2)
          (Rendering|Material|SetMaterial _floorceiling_mesh _index_2 (Rendering|Material|GetMaterial (LocalVariables|GetNew_mesh) _index_2)))
        (Variables|Mesh|SetRevert%20Default%20Materials false)))))