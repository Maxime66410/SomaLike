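; BP_Door_main is a hinged door for the suburb house pack that toggles open and closed through OpenClose unless locked.
; A dot product between the player-to-door direction and the root's forward vector picks the swing side, so the timeline-driven yaw reaches 90 degrees either way.
; Closing reverses the timeline.
; The construction script sets the mesh from the DoorsMain selection and can restore its default materials via a self-resetting flag.
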(event Custom|OpenClose
  (bind _defaultsceneroot (Variables|Default|GetDefaultSceneRoot))
  (if (not (Variables|Mesh|GetLocked))
    (if (Variables|Default|GetDoorClosed)
      (Variables|Default|SetDoorClosed false)
      (Variables|Default|SetDotProduct (Math|Vector|DotProduct (Math|Vector|Normalize (- (Transformation|GetWorldLocation _defaultsceneroot) (Transformation|GetActorLocation (Game|GetPlayerCharacter 0)))) (Math|Vector|GetForwardVector _defaultsceneroot)))
      (bind (_direction _openclose) (Timeline|Door_openclose Play)
        (:Update
          (Transformation|SetRelativeRotation (Variables|Default|GetDoor_mesh) (Math|Rotator|MakeRotator 0.0 0.0 (Math|Float|Lerp 0.0 (Math|Float|SelectFloat 9e+01 -9e+01 (>= (Variables|Default|GetDotProduct) 0.0)) _openclose)) false false))
        (:Finished
          (switch Utilities|FlowControl|Switch|SwitchonETimelineDirection _direction
            (:Backward
              (Variables|Default|SetDoorClosed true)))))
      (else
        (Timeline|Door_openclose Reverse)))))

(event EventBeginPlay)

(fn ConstructionScript
  (bind _doors_main (Variables|Mesh|GetDoors_main))
  (bind _door_mesh (Variables|Default|GetDoor_mesh))
  (bind _door_meshes (Variables|Mesh|GetDoor%20Meshes))
  (bind _returnvalue (Rendering|Material|GetNumMaterials _door_mesh))
  (bind _returnvalue_2 (Math|Conversions|ToInteger(Byte) _doors_main))
  (bind _output (Utilities|Array|Get(acopy) _door_meshes _returnvalue_2))
  (Components|StaticMesh|SetStaticMesh (Variables|Default|GetDoor_mesh) _output)
  (LocalVariables|SetNew_mesh _output)
  (if (Variables|Mesh|GetRevert%20Default%20Materials)
    (LocalVariables|SetNumber%20Of%20Materials _returnvalue)
    (for _index (range 0 _returnvalue)
      (Rendering|Material|SetMaterial _door_mesh _index (Rendering|Material|GetMaterial (LocalVariables|GetNew_mesh) _index)))
    (Variables|Mesh|SetRevert%20Default%20Materials false)))