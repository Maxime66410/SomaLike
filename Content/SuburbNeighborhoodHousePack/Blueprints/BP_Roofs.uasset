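; BP_Roofs is a modular roof piece for the suburban house pack, with its variant chosen by the Roofs enum.
; The construction script uses the enum as an index into RoofMeshes to set the roof mesh.
; Window variants also get a matching glass mesh, while all other listed variants destroy the Windowglass component.
; RevertDefaultMaterials acts as a one-shot toggle that restores the mesh's default materials, then clears itself.
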(event EventBeginPlay)

(event Collision|EventActorBeginOverlap
  (params (OtherActor :type Actor%20Object%20Reference)))

(event EventTick
  (params (DeltaSeconds :type Float%20%28single-precision%29)))

(fn ConstructionScript
  (bind _roofs (Variables|Mesh|GetRoofs))
  (bind _roof_meshes (Variables|Mesh|GetRoof%20Meshes))
  (bind _roof_mesh (Variables|Default|GetRoof_mesh))
  (bind _windowglass (Variables|Default|GetWindowglass))
  (bind _returnvalue (Math|Conversions|ToInteger(Byte) _roofs))
  (bind _output (Utilities|Array|Get(acopy) _roof_meshes _returnvalue))
  (Components|StaticMesh|SetStaticMesh (Variables|Default|GetRoof_mesh) _output)
  (LocalVariables|SetNew_mesh _output)
  (switch Utilities|FlowControl|Switch|SwitchonE_Roofs _roofs
    (:NewEnumerator19
      (Components|DestroyComponent _windowglass :!label _label))
    (:NewEnumerator5
      (goto _label))
    (:NewEnumerator6
      (goto _label))
    (:NewEnumerator7
      (Components|StaticMesh|SetStaticMesh _windowglass "/Game/SuburbNeighborhoodHousePack/Meshes/Meshes_construction/SM_Roof_5x_end_window_windowglass.SM_Roof_5x_end_window_windowglass"))
    (:NewEnumerator8
      (goto _label))
    (:NewEnumerator9
      (goto _label))
    (:NewEnumerator2
      (goto _label))
    (:NewEnumerator20
      (Components|StaticMesh|SetStaticMesh _windowglass "/Game/SuburbNeighborhoodHousePack/Meshes/Meshes_construction/SM_Roof_7x_end_window_A_windowglass.SM_Roof_7x_end_window_A_windowglass"))
    (:NewEnumerator3
      (goto _label))
    (:NewEnumerator4
      (goto _label))
    (:NewEnumerator10
      (goto _label))
    (:NewEnumerator11
      (Components|StaticMesh|SetStaticMesh _windowglass "/Game/SuburbNeighborhoodHousePack/Meshes/Meshes_construction/SM_Roof_8x_end_window_A_windowglass.SM_Roof_8x_end_window_A_windowglass"))
    (:NewEnumerator12
      (goto _label))
    (:NewEnumerator14
      (goto _label))
    (:NewEnumerator15
      (goto _label))
    (:NewEnumerator16
      (goto _label))
    (:NewEnumerator22
      (goto _label))
    (:NewEnumerator13
      (goto _label))
    (:NewEnumerator17
      (goto _label))
    (:NewEnumerator18
      (goto _label))
    (:NewEnumerator21
      (goto _label))
    (:NewEnumerator0
      (goto _label))
    (:NewEnumerator1
      (Components|StaticMesh|SetStaticMesh _windowglass "/Game/SuburbNeighborhoodHousePack/Meshes/Meshes_construction/SM_Roof_Extra_Window_Double_windowglass.SM_Roof_Extra_Window_Double_windowglass"))
    (:NewEnumerator23
      (Components|StaticMesh|SetStaticMesh _windowglass "/Game/SuburbNeighborhoodHousePack/Meshes/Meshes_construction/SM_Roof_Extra_Window_Single_windowglass.SM_Roof_Extra_Window_Single_windowglass")))
  (if (Variables|Mesh|GetRevert%20Default%20Materials)
    (bind _output_get (LocalVariables|SetNumber%20Of%20Materials (Rendering|Material|GetNumMaterials _roof_mesh)))
    (for _index (range 0 _output_get)
      (Rendering|Material|SetMaterial _roof_mesh _index (Rendering|Material|GetMaterial (LocalVariables|GetNew_mesh) _index)))
    (Variables|Mesh|SetRevert%20Default%20Materials false)))